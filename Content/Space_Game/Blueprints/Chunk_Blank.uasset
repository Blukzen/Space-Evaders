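; Level chunk actor for the space game that triggers loading of the next chunk as the Space_Ship passes through.
; Overlapping its Trigger calls LoadNewChunk on SpaceGamemode, then the chunk destroys itself after a short delay.
; GetSpawnPosition exposes a world transform from its SpawnPosition component.
; SpawnObstacles adds one Obstacle1 child actor, placed by the SpawnObstacle helper around ObstacleSpawnPosition, but is not called within this Blueprint.
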(event `self.Trigger.OnComponentBeginOverlap`
  (params (OverlappedComponent :type "PrimitiveComponent Object Reference") (OtherActor :type "Actor Object Reference") (OtherComp :type "PrimitiveComponent Object Reference") (OtherBodyIndex :type Integer) (bFromSweep :type Boolean) (SweepResult :type "HitResult Structure (by ref)"))
  (cast `/Game/Space_Game/Blueprints/Space_Ship` OtherActor)
  (bind _asspace_gamemode (cast `/Game/Space_Game/SpaceGamemode` (`GameplayStatics.GetGameMode`)))
  (`/Game/Space_Game/SpaceGamemode.LoadNewChunk` _asspace_gamemode)
  (`KismetSystemLibrary.Delay` 1.0)
  (`self.K2_DestroyActor`))

(fn `GetSpawnPosition`
  (returns (SpawnPosition :type "Transform Structure"))
  (return (`SceneComponent.K2_GetComponentToWorld` (`self.SpawnPosition`))))

(fn `SpawnObstacles`
  (bind _returnvalue (`SpaceshipAccelerateBPLibrary.SpawnObstacle` (`SceneComponent.GetRelativeTransform` (`self.ObstacleSpawnPosition`)) 6000 3000 5 10))
  (bind _returnvalue_2 (`AddComponent|NODE_AddChildActorComponent-1` :`RelativeTransform` _returnvalue))
  (`ChildActorComponent.SetChildActorClass` _returnvalue_2 "/Game/Space_Game/Blueprints/Obstacle1.Obstacle1_C"))

(fn `UserConstructionScript`)