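; Player spaceship that flies forward along X at ever-increasing speed, steers sideways and reports its X position as score.
; Left and Right axes share one path that sets Y velocity and eases the ship into a bank proportional to it.
; Tick drives forward velocity and writes a speed-derived DifficultyMultiplier to SpaceGamemode.
; That multiplier feeds back to reduce acceleration in steps until speed levels off.
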(event `InputAxis|Left`
  (params (AxisValue :type "Float (single-precision)"))
  (bind _charactermovement (`self.CharacterMovement`))
  (set `MovementComponent.Velocity` (`KismetMathLibrary.MakeVector` (.x (`MovementComponent.Velocity` _charactermovement)) (* (`self.TurnSpeed`) (+ (stale `InputAxis|Right` AxisValue) AxisValue))) _charactermovement :!label _label)
  (`self.K2_SetActorRotation` (`KismetMathLibrary.RLerp` (`self.K2_GetActorRotation`) (`KismetMathLibrary.MakeRotator` (* (/ (.y (`self.GetVelocity`)) 4000.0) 45.0)) 0.05)))

(event `InputAxis|Right`
  (params (AxisValue :type "Float (single-precision)"))
  (goto _label))

(event `self.ReceiveBeginPlay`
  (set `self.BaseSpeed` 500.0)
  (set `self.TurnSpeed` 4000.0))

(event `self.ReceiveTick`
  (params (DeltaSeconds :type "Float (single-precision)"))
  (bind _charactermovement (`self.CharacterMovement`))
  (set `MovementComponent.Velocity` (`KismetMathLibrary.MakeVector` (`self.BaseSpeed`) (.y (`MovementComponent.Velocity` _charactermovement)) (.z (`MovementComponent.Velocity` _charactermovement))) _charactermovement)
  (bind _asspace_gamemode (cast `/Game/Space_Game/SpaceGamemode` (`GameplayStatics.GetGameMode`)))
  (bind _output_get (set `self.BaseSpeed` (+ (`self.BaseSpeed`) (* (- 4.0 (`KismetMathLibrary.Conv_IntToDouble` (`/Game/Space_Game/SpaceGamemode.DifficultyMultiplier` _asspace_gamemode))) 1.0))))
  (`self.SetDifficultyMultiplier` _output_get))

(fn `GetScore`
  (returns (NewParam :type Integer))
  (return (`KismetMathLibrary.Round` (.x (`self.K2_GetActorLocation`)))))

(fn `SetDifficultyMultiplier`
  (params (CurrentSpeed :type "Float (double-precision)"))
  (bind _asspace_gamemode (cast `/Game/Space_Game/SpaceGamemode` (`GameplayStatics.GetGameMode`)))
  (set `/Game/Space_Game/SpaceGamemode.DifficultyMultiplier` (`KismetMathLibrary.FTrunc` (* (/ CurrentSpeed 20000.0) 4.0)) _asspace_gamemode))

(fn `UserConstructionScript`)