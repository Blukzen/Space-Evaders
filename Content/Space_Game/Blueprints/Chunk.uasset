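; Chunk is a level segment actor for a space ship game that fills itself with obstacles and chains to the next segment.
; Its construction script adds randomly chosen obstacle child actors at generated transforms around a spawn point, their count scaling with the game mode's difficulty up to a cap.
; When the ship overlaps its trigger, it asks the game mode to load a new chunk, then destroys itself after a short delay.
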(event `self.Trigger.OnComponentBeginOverlap`
  (params (OverlappedComponent :type "PrimitiveComponent Object Reference") (OtherActor :type "Actor Object Reference") (OtherComp :type "PrimitiveComponent Object Reference") (OtherBodyIndex :type Integer) (bFromSweep :type Boolean) (SweepResult :type "HitResult Structure (by ref)"))
  (cast `/Game/Space_Game/Blueprints/Space_Ship` OtherActor)
  (bind _asspace_gamemode (cast `/Game/Space_Game/SpaceGamemode` (`GameplayStatics.GetGameMode`)))
  (`/Game/Space_Game/SpaceGamemode.LoadNewChunk` _asspace_gamemode)
  (`KismetSystemLibrary.Delay` 1.0)
  (`self.K2_DestroyActor`))

(fn `GetSpawnPosition`
  (returns (SpawnPosition :type "Transform Structure"))
  (return (`SceneComponent.K2_GetComponentToWorld` (`self.SpawnPosition`))))

(fn `SpawnObstacles`
  (bind _obstacles (`self.Obstacles`))
  (bind _returnvalue (`SpaceshipAccelerateBPLibrary.SpawnObstacle` (`SceneComponent.GetRelativeTransform` (`self.ObstacleSpawnPosition`)) 6000 1000 10 15))
  (bind _returnvalue_2 (`AddComponent|NODE_AddChildActorComponent-1` :`RelativeTransform` _returnvalue))
  (`ChildActorComponent.SetChildActorClass` _returnvalue_2 (`|GetArrayItem` _obstacles (`KismetMathLibrary.RandomIntegerInRange` 0 (`KismetArrayLibrary.Array_LastIndex` _obstacles)))))

(fn `UserConstructionScript`
  (bind _asspace_gamemode (cast `/Game/Space_Game/SpaceGamemode` (`GameplayStatics.GetGameMode`)))
  (for _ (range (+ (`KismetMathLibrary.Min` (`KismetMathLibrary.Max` (- (`/Game/Space_Game/SpaceGamemode.DifficultyMultiplier` _asspace_gamemode) 1)) 3) 1))
    (`self.SpawnObstacles`)))